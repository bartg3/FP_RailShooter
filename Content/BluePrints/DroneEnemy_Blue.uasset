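; Blue drone enemy actor that drifts between two move points, spins, and can fire projectiles at the player.
; FindNewLocation re-runs after a random delay, picking a random point and yaw speed that Tick applies to the Sphere.
; Moving re-arms a short timer, lerping from the current location by a small fixed alpha for eased motion.
; ShootAtPlayer faces the player pawn and spawns EnemyProjectile at the Arrow, with no caller in this graph.
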(event `self.ReceiveBeginPlay`
  (`self.FindNewLocation`)
  (`KismetSystemLibrary.Delay` 2.0))

(event `Moving`
  (bind _sphere (`self.Sphere`))
  (set `self.Alpha` 0.0)
  (`KismetSystemLibrary.K2_SetTimerDelegate` (delegate `Moving`) 0.02)
  (set `self.Alpha` (+ (`self.Alpha`) 0.02))
  (`SceneComponent.K2_SetWorldLocation` _sphere (`KismetMathLibrary.VLerp` (`SceneComponent.K2_GetComponentLocation` _sphere) (`self.LocationToMove`) (`self.Alpha`)) false false))

(event `self.ReceiveTick`
  (params (DeltaSeconds :type "Float (single-precision)"))
  (`SceneComponent.K2_AddLocalRotation` (`self.Sphere`) (`KismetMathLibrary.MakeRotator` 0.0 0.0 (`self.Delta Rotation Z (Yaw)`)) false false))

(event `FindNewLocation`
  (bind _array (`|MakeArray` (`self.MoveLocation1`) (`self.MoveLocation2`)))
  (set `self.Delta Rotation Z (Yaw)` (`KismetMathLibrary.RandomFloatInRange` -1.0 1.0))
  (set `self.LocationToMove` (`SceneComponent.K2_GetComponentLocation` (`|GetArrayItem` _array (`KismetMathLibrary.RandomIntegerInRange` 0 (`KismetArrayLibrary.Array_LastIndex` _array)))))
  (`self.Moving`)
  (`KismetSystemLibrary.Delay` (`KismetMathLibrary.RandomFloatInRange` 15.0 18.0))
  (`self.FindNewLocation`))

(event `ShootAtPlayer`
  (bind _sphere (`self.Sphere`))
  (`SceneComponent.K2_SetWorldRotation` _sphere (`KismetMathLibrary.FindLookAtRotation` (`SceneComponent.K2_GetComponentLocation` _sphere) (`SceneComponent.K2_GetComponentLocation` (`Actor.RootComponent` (`GameplayStatics.GetPlayerPawn` 0)))) false false)
  (`|SpawnActorFromClass` "/Game/BluePrints/EnemyProjectile.EnemyProjectile_C" (`SceneComponent.K2_GetComponentToWorld` (`self.Arrow`)) "Undefined" "OverrideRootScale" null null))

(fn `UserConstructionScript`)