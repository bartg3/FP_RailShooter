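; HealthPickup is a spinning pickup actor that releases a HealthProjectile when its GainHealth event is called.
; Tick yaws the Cube by a fixed step each frame, independent of delta time.
; GainHealth turns the Cube to face the first player's pawn, spawns the projectile at the Arrow's transform, then destroys the pickup.
; Nothing in this Blueprint calls GainHealth, and its overlap event is empty.
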(event `GainHealth`
  (bind _cube (`self.Cube`))
  (`SceneComponent.K2_SetWorldRotation` _cube (`KismetMathLibrary.FindLookAtRotation` (`SceneComponent.K2_GetComponentLocation` _cube) (`SceneComponent.K2_GetComponentLocation` (`Actor.RootComponent` (`GameplayStatics.GetPlayerPawn` 0)))) false false)
  (`|SpawnActorFromClass` "/Game/BluePrints/HealthProjectile.HealthProjectile_C" (`SceneComponent.K2_GetComponentToWorld` (`self.Arrow`)) "Undefined" "OverrideRootScale" null null)
  (`self.K2_DestroyActor`))

(event `self.ReceiveActorBeginOverlap`
  (params (OtherActor :type "Actor Object Reference")))

(event `self.ReceiveTick`
  (params (DeltaSeconds :type "Float (single-precision)"))
  (`SceneComponent.K2_AddLocalRotation` (`self.Cube`) (`KismetMathLibrary.MakeRotator` 0.0 0.0 1.0) false false))

(fn `UserConstructionScript`)