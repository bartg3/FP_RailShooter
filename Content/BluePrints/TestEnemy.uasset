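; TestEnemy is a test enemy actor whose Cube shuttles endlessly between two marker components from BeginPlay.
; MoveComponentTo moves it to MoveLocation's relative location and world rotation, then back to OriginalLocation without copying that marker's rotation.
; MoveTime sets both travel durations, WaitTime the pause at the far end, and a fixed delay precedes each repeat.
; EnemyStart is empty and the DestroyActor call is unconnected.
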(event `EnemyStart`)

(event `self.ReceiveBeginPlay`
  (bind _cube (`self.Cube`))
  (bind _movelocation (`self.MoveLocation`))
  (`KismetSystemLibrary.MoveComponentTo` _cube (`SceneComponent.RelativeLocation` _movelocation) (`SceneComponent.K2_GetComponentRotation` _movelocation) false false (`self.MoveTime`) :!label _label)
  (`KismetSystemLibrary.Delay` (`self.WaitTime`))
  (`KismetSystemLibrary.MoveComponentTo` _cube (`SceneComponent.RelativeLocation` (`self.OriginalLocation`)) (struct) false false (`self.MoveTime`))
  (`KismetSystemLibrary.Delay` 2.0)
  (goto _label))

(fn `UserConstructionScript`)